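; Electrocute gameplay ability that, as it stands, handles only targeting and the input hold, with no damage or effects yet.
; On activation, a target-data-under-mouse task supplies a hit result, which is stored along with the owner's references.
; The mouse cursor is then hidden until a wait-for-input-release task fires and ends the ability, with debug prints around the wait.
; Ending the ability also restores the cursor.
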(event Ability|EventActivateAbility
  (bind _datahandle (|TargetDataUnderMouse)
    (:ValidData
      (Class|DntBeamSpell|StoreMouseDataInfo (Ability|TargetData|GetHitResultfromTargetData _datahandle))
      (Class|DntBeamSpell|StoreOwnerVariables)
      (Utilities|FlowControl|Sequence
        (:then_0
          (Variables|/Script/Engine.PlayerController|SetbShowMouseCursor (Variables|Default|GetOwnerPlayerController) false))
        (:then_1
          (Development|PrintString "准备进入 Wait 节点" true true "(R=1.000000,G=0.994862,B=0.000000,A=1.000000)")
          (Ability|Tasks|WaitInputRelease true
            (:OnRelease
              (Development|PrintString "成功捕获 Release" true true "(R=0.000000,G=1.000000,B=0.014935,A=1.000000)")
              (Variables|/Script/Engine.PlayerController|SetbShowMouseCursor (Variables|Default|GetOwnerPlayerController) true)
              (Ability|EndAbility))))))))

(event Ability|EventOnEndAbility
  (params (bWasCancelled :type Boolean))
  (Variables|/Script/Engine.PlayerController|SetbShowMouseCursor (Variables|Default|GetOwnerPlayerController) true))